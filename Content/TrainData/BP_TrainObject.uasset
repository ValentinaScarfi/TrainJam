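; BP_TrainObject is a train data object that derives a train's direction and list of stations from its start and terminate stations.
; GetDirection sets Northbound when TerminateStation precedes StartStation in the E_Stations enum order.
; FindRoute uses that flag to order the loop bounds, then casts each index to E_Stations and appends it to Route.
; Both branches count upward, so Route follows enum order rather than travel order.
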(fn `FindRoute`
  (bind (_train_trainnumber _train_trainlength _train_traincolor _train_traincompany _train_capacity _train_startstation _train_terminatestation) (break `/Game/TrainData/Struct_Train` (`self.Train`)))
  (bind (_train_trainnumber_2 _train_trainlength_2 _train_traincolor_2 _train_traincompany_2 _train_capacity_2 _train_startstation_2 _train_terminatestation_2) (break `/Game/TrainData/Struct_Train` (`self.Train`)))
  (if (`self.Northbound`)
    ;[1 1 1] If Northbound != true
    (for _index (range (`KismetMathLibrary.Conv_ByteToInt` _train_terminatestation_2) (+ (`KismetMathLibrary.Conv_ByteToInt` _train_startstation_2) 1))
      (`KismetArrayLibrary.Array_Add` (`self.Route`) (cast `/Game/TrainData/E_Stations` (`KismetMathLibrary.Conv_IntToByte` _index))))
    (else
      ;[1 1 1] If Northbound == true
      (for _index_2 (range (`KismetMathLibrary.Conv_ByteToInt` _train_startstation) (+ (`KismetMathLibrary.Conv_ByteToInt` _train_terminatestation) 1))
        (`KismetArrayLibrary.Array_Add` (`self.Route`) (cast `/Game/TrainData/E_Stations` (`KismetMathLibrary.Conv_IntToByte` _index_2)))))))

(fn `GetDirection`
  (bind (_train_trainnumber _train_trainlength _train_traincolor _train_traincompany _train_capacity _train_startstation _train_terminatestation) (break `/Game/TrainData/Struct_Train` (`self.Train`)))
  (set `self.Northbound` (< _train_terminatestation _train_startstation)))