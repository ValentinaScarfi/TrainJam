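; Train control-room puzzle manager that randomly generates instruction rules on BeginPlay, currently output only as debug prints.
; Each of two slots draws three distinct instruction categories and picks one.
; GetStructInformation iterates that category's values, such as stations, weather or time windows, calling GenerateInput for each.
; GenerateInput uses the slot number to produce random console colours or platform switch patterns, re-rolling duplicate patterns.
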(event `self.ReceiveBeginPlay`
  (`/Engine/EditorBlueprintResources/StandardMacros.IncrementInt` (`self.CurrentInstruction`)
    (:`  `
      (bind _setofchoseninstructionsstrings (`self.PopulateInstructionSlot` 3))
      (bind _choseninstruction (`self.PickRandomInstructionForSlot` _setofchoseninstructionsstrings))
      (`KismetSystemLibrary.PrintString` _choseninstruction true true (struct :`G` 0.66 :`B` 1.0 :`A` 1.0) 60.0)
      (`self.GetStructInformation` _choseninstruction)
      (`KismetSystemLibrary.PrintString` "Which switches need to be pressed is determined by the " true true (struct :`R` 1.0 :`G` 0.988632 :`A` 1.0) 60.0)
      (`/Engine/EditorBlueprintResources/StandardMacros.IncrementInt` (`self.CurrentInstruction`)
        (:`  `
          (bind _setofchoseninstructionsstrings_2 (`self.PopulateInstructionSlot` 3))
          (bind _choseninstruction_2 (`self.PickRandomInstructionForSlot` _setofchoseninstructionsstrings_2))
          (`KismetSystemLibrary.PrintString` _choseninstruction_2 true true (struct :`G` 0.66 :`B` 1.0 :`A` 1.0) 60.0)
          (`self.GetStructInformation` _choseninstruction_2)
          (`/Engine/EditorBlueprintResources/StandardMacros.IncrementInt` (`self.CurrentInstruction`)))))))

(fn `Generate3Colours`
  (params (ListOfColours :type "Array of Color Structure"))
  (returns (ChosenColours :type "Array of Color Structure"))
  (locals (SetOfColours :type "Array of Color Structure"))
  (bind _setofcolours (`local.SetOfColours`))
  (for _ (range 3)
    (`KismetArrayLibrary.Array_Add` _setofcolours (`|GetArrayItem` ListOfColours (`KismetMathLibrary.RandomIntegerInRange` 0 (- (`KismetArrayLibrary.Array_Length` ListOfColours) 1)))))
  (return _setofcolours))

(fn `GenerateInput`
  (locals (ControlRoomButtonConsole :type "Array of Color Structure") (LockerCombination :type "Array of Integer"))
  (bind _setofplatformsswitches (`self.SetOfPlatformsSwitches`))
  (switch `int` (`self.CurrentInstruction`)
    (:`1`
      (bind _chosencolours (`self.Generate3Colours` (`local.ControlRoomButtonConsole`)))
      (for _array_element _chosencolours
        (`KismetSystemLibrary.PrintString` "ThisColour" true true (`KismetMathLibrary.Conv_ColorToLinearColor` _array_element) 60.0)))
    (:`2`
      (bind _newplatformsswitches (`self.GeneratePlatformSwitches` :!label _label))
      (if (`KismetArrayLibrary.Array_Contains` _setofplatformsswitches _newplatformsswitches)
        (goto _label)
        (else
          (`KismetArrayLibrary.Array_Add` _setofplatformsswitches _newplatformsswitches)
          (bind (_1 _2 _3 _4) (break `/Game/TrainData/Struct_Platform` _newplatformsswitches))
          (`KismetSystemLibrary.PrintString` (`KismetStringLibrary.Conv_BoolToString` _1) true true (struct :`G` 0.66 :`B` 1.0 :`A` 1.0) 60.0)
          (`KismetSystemLibrary.PrintString` (`KismetStringLibrary.Conv_BoolToString` _2) true true (struct :`G` 0.66 :`B` 1.0 :`A` 1.0) 60.0)
          (`KismetSystemLibrary.PrintString` (`KismetStringLibrary.Conv_BoolToString` _3) true true (struct :`G` 0.66 :`B` 1.0 :`A` 1.0) 60.0)
          (`KismetSystemLibrary.PrintString` (`KismetStringLibrary.Conv_BoolToString` _4) true true (struct :`G` 0.66 :`B` 1.0 :`A` 1.0) 60.0))))))

(fn `GeneratePlatformSwitches`
  (returns (newPlatformsSwitches :type "/Game/TrainData/Struct_Platform Structure"))
  (return (make `/Game/TrainData/Struct_Platform` (`KismetMathLibrary.RandomBool`) (`KismetMathLibrary.RandomBool`) (`KismetMathLibrary.RandomBool`) (`KismetMathLibrary.RandomBool`))))

(fn `GetStructInformation`
  (params (InstructionString :type String))
  (locals (DepartureStation :type "/Game/TrainData/E_Stations Enum") (PlatformsAvailable :type "Array of Integer"))
  (switch `string` InstructionString
    (:`Departure Station`
      (bind _enumvalue (foreach `/Game/TrainData/E_Stations` :!label _label)
        (:`LoopBody`
          (`KismetSystemLibrary.PrintString` (`|GetEnumeratorNameAsString` _enumvalue) true true (struct :`R` 0.936638 :`G` 1.0 :`B` 0.990007 :`A` 1.0) 60.0)
          (`self.GenerateInput` :!label _label_2))))
    (:`Time`
      (`self.TimeInstructions` 3))
    (:`Company`
      (bind _enumvalue_2 (foreach `/Game/TrainData/E_TrainCompanies`)
        (:`LoopBody`
          (`KismetSystemLibrary.PrintString` (`|GetEnumeratorNameAsString` _enumvalue_2) true true (struct :`R` 0.936638 :`G` 1.0 :`B` 0.990007 :`A` 1.0) 60.0)
          (goto _label_2))))
    (:`Platform`
      (for _array_element (`local.PlatformsAvailable`)
        (`KismetSystemLibrary.PrintString` (`KismetStringLibrary.Conv_IntToString` _array_element) true true (struct :`R` 0.936638 :`G` 1.0 :`B` 0.990007 :`A` 1.0) 60.0)
        (goto _label_2)))
    (:`Colour`
      (bind _enumvalue_3 (foreach `/Game/TrainData/E_TrainColors`)
        (:`LoopBody`
          (`KismetSystemLibrary.PrintString` (`|GetEnumeratorNameAsString` _enumvalue_3) true true (struct :`R` 0.936638 :`G` 1.0 :`B` 0.990007 :`A` 1.0) 60.0)
          (goto _label_2))))
    (:`Arrival Station`
      (goto _label))
    (:`Weather`
      (bind _enumvalue_4 (foreach `/Game/TrainData/E_Weather`)
        (:`LoopBody`
          (`KismetSystemLibrary.PrintString` (`|GetEnumeratorNameAsString` _enumvalue_4) true true (struct :`R` 0.936638 :`G` 1.0 :`B` 0.990007 :`A` 1.0) 60.0)
          (goto _label_2))))))

(fn `PickRandomInstructionForSlot`
  (params (SetOfInstructions :type "Array of String"))
  (returns (ChosenInstruction :type String))
  (return (`|GetArrayItem` SetOfInstructions (`KismetMathLibrary.RandomIntegerInRange` 0 (- (`KismetArrayLibrary.Array_Length` SetOfInstructions) 1)))))

(fn `PopulateInstructionSlot`
  (params (HowManyPerSlot :type Integer :default 3))
  (returns (SetOfChosenInstructionsStrings :type "Array of String"))
  (locals (RandomInstructions :type "Array of Integer") (InstructionsString :type "Array of String") (OutputStrings :type "Array of String"))
  (bind _returnvalue (`KismetMathLibrary.RandomIntegerInRange` 0 8))
  (bind _randominstructions (`local.RandomInstructions`))
  (set `self.InstructionsStrings` (`local.InstructionsString`))
  (while (!= (`KismetArrayLibrary.Array_Length` (`local.RandomInstructions`)) HowManyPerSlot)
    (if (not (`KismetArrayLibrary.Array_Contains` _randominstructions _returnvalue))
      (`KismetArrayLibrary.Array_AddUnique` _randominstructions _returnvalue)))
  (for _array_element (`local.RandomInstructions`)
    (`KismetArrayLibrary.Array_AddUnique` (`local.OutputStrings`) (`|GetArrayItem` (`local.InstructionsString`) _array_element)))
  (return (`local.OutputStrings`)))

(fn `TimeInstructions`
  (params (NumberOfTimeConditions :type Integer))
  (for _index (range 1 (+ NumberOfTimeConditions 1))
    (switch `int` _index
      (:`1`
        (`KismetSystemLibrary.PrintString` "Before 11" true true (struct :`R` 1.0 :`B` 0.054731 :`A` 1.0) 60.0))
      (:`2`
        (`KismetSystemLibrary.PrintString` "Between 11.05 and 2.00" true true (struct :`R` 1.0 :`B` 0.015782 :`A` 1.0) 60.0))
      (:`3`
        (`KismetSystemLibrary.PrintString` "After 2.05" true true (struct :`R` 1.0 :`G` 0.014146 :`A` 1.0) 60.0)))
    (`self.GenerateInput`)))

(fn `UserConstructionScript`)