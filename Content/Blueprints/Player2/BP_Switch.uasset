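; Colour-coded push-button switch for Player 2 that submits its colour to the character's instruction checker when interacted with.
; A press also fires the AnimateTrain dispatcher, plays a sound and runs a timeline that slides the button along local X.
; The construction script builds a dynamic material from the per-instance Colour.
; Box overlap by the Player 2 character swaps that material for a flat base one until the overlap ends.
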(event `self.ReceiveBeginPlay`
  ;[1 1 1] Set Button relative position for animation
  (set `self.StartPos` (`SceneComponent.RelativeLocation` (`self.Switch`))))

(event `ButtonPressed`
  (bind _startpos (`self.StartPos`))
  (bind _asbp_character_player_2 (cast `/Game/Blueprints/Player2/BP_CharacterPlayer2` (`GameplayStatics.GetPlayerCharacter` 0)))
  (`/Game/TrainData/BP_InstructionChecker.AddColourToList` (`/Game/Blueprints/Player2/BP_CharacterPlayer2.InstructionCheckerRef` _asbp_character_player_2) (`self.Colour`))
  ;[1 1 1] Call event dispatch
  (`self.AnimateTrain`)
  ;[1 1 1] Animate Button Press
  (bind (_direction _speed) (`Timeline|ButtonAnim` :!via `PlayFromStart`)
    (:`Update`
      (`SceneComponent.K2_SetRelativeLocation` (`self.Switch`) (`KismetMathLibrary.VLerp` _startpos (`KismetMathLibrary.MakeVector` -2.0 (.y _startpos) (.z _startpos)) _speed) false false))))

(event `self.Box.OnComponentBeginOverlap`
  (params (OverlappedComponent :type "PrimitiveComponent Object Reference") (OtherActor :type "Actor Object Reference") (OtherComp :type "PrimitiveComponent Object Reference") (OtherBodyIndex :type Integer) (bFromSweep :type Boolean) (SweepResult :type "HitResult Structure (by ref)"))
  ;[1 1 1] Overlap Event to Change Colour
  (cast `/Game/Blueprints/Player2/BP_CharacterPlayer2` OtherActor)
  (`PrimitiveComponent.SetMaterial` (`self.Switch`) 0 "/Game/Assets/Material/M_FlatBase.M_FlatBase"))

(event `self.Box.OnComponentEndOverlap`
  (params (OverlappedComponent :type "PrimitiveComponent Object Reference") (OtherActor :type "Actor Object Reference") (OtherComp :type "PrimitiveComponent Object Reference") (OtherBodyIndex :type Integer))
  ;[1 1 1] Overlap Event to Change Colour
  (cast `/Game/Blueprints/Player2/BP_CharacterPlayer2` OtherActor)
  (`PrimitiveComponent.SetMaterial` (`self.Switch`) 0 (`self.Dynamic Material`)))

(fn `Interact`
  (params (TargetPoint :type "SceneComponent Object Reference"))
  (returns (Val :type Boolean))
  (`self.ButtonPressed`)
  (`GameplayStatics.PlaySoundAtLocation` "/Game/Assets/Audio/switch-2.switch-2" (`self.K2_GetActorLocation`))
  (return false))

(fn `UserConstructionScript`
  ;[1 1 1] Allow Colour of button to be editable per instance using Dynamic Material Instance
  (bind _returnvalue (`PrimitiveComponent.CreateDynamicMaterialInstance` (`self.Switch`) 0 "/Game/Assets/Material/M_FlatWallRed.M_FlatWallRed"))
  (bind _output_get (set `self.Dynamic Material` _returnvalue))
  (`MaterialInstanceDynamic.SetVectorParameterValue` _output_get "Colour" (`self.Colour`)))