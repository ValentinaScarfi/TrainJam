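; BP_TrainModel is a train actor that animates a train's arrival along the Y axis.
; AnimateIn maps the arrival status to a spawn transform and final Y position for northbound, southbound or either of two terminating cases.
; It spawns a new instance of its own class there, and a timeline lerps that instance to the final position.
; A steam sound plays at the train's location when the movement finishes.
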(event `self.ReceiveTick`
  (params (DeltaSeconds :type "Float (single-precision)")))

(event `AnimateIn`
  (params (ArrivalStatus :type "/Game/Blueprints/Player2/E_ArrivalStatus Enum" :default "NewEnumerator0"))
  (bind _traintransform_location (`KismetMathLibrary.BreakTransform` (`self.TrainTransform`)))
  ;[1 1 1] Set spawn position and final position on Y axis to lerp to
  (if (`|EnumEquality` ArrivalStatus "NewEnumerator2")
    (set `self.TrainTransform` (`self.NorthboundTransform`))
    (set `self.FinalPos` (`self.NorthboundFinal`))
    (bind _returnvalue (`|SpawnActorFromClass` "BP_TrainModel_C" (`self.TrainTransform`) "Undefined" "OverrideRootScale" null null :!label _label))
    ;[1 1 1] Animate Train In
    (bind (_direction _positiony) (`Timeline|AnimateTrain` :!via `PlayFromStart`)
      (:`Update`
        (`SceneComponent.K2_SetWorldLocation` (`Actor.RootComponent` _returnvalue) (`KismetMathLibrary.VLerp` _traintransform_location (`KismetMathLibrary.MakeVector` (.x _traintransform_location) (`self.FinalPos`) (.z _traintransform_location)) _positiony) false false))
      (:`Finished`
        (`GameplayStatics.PlaySoundAtLocation` "/Game/StarterContent/Audio/Steam01.Steam01" (`self.K2_GetActorLocation` _returnvalue))))
    (elif (`|EnumEquality` ArrivalStatus "NewEnumerator3")
      (set `self.TrainTransform` (`self.SoutboundTransform`))
      (set `self.FinalPos` (`self.SouthboundFinal`))
      (goto _label)
      (elif (`|EnumEquality` ArrivalStatus "NewEnumerator0")
        (set `self.TrainTransform` (`self.NorthTermTransform`))
        (set `self.FinalPos` (`self.NorthTermFinal`))
        (goto _label)
        (elif (`|EnumEquality` ArrivalStatus "NewEnumerator1")
          (set `self.TrainTransform` (`self.SouthTermTransform`))
          (set `self.FinalPos` (`self.SouthTermFinal`))
          (goto _label))))))

(fn `UserConstructionScript`)