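; Station manager that works out how a train arrives at a station and spawns its visual model.
; TrainArrival classifies the train as terminating or through in either direction, using its Westbound flag and last route stop.
; SpawnTrainModel maps that status to a north/south spawn transform plus arrival and departure targets, then spawns BP_TrainModel.
; The EventGraph chain feeding both into the model's AnimateIn is unconnected and never runs.
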(fn `SpawnTrainModel`
  (params (ArrivalStatus :type "/Game/Blueprints/Player2/E_ArrivalStatus Enum" :default "NewEnumerator0"))
  (returns (SpawnedTrainObject :type "/Game/Blueprints/Player2/BP_TrainModel Object Reference") (TrainSpawnTransform :type "Transform Structure") (ArrivalTargetPos :type "Float (double-precision)") (DepartureTargetPos :type "Float (double-precision)"))
  (bind _trainspawntransform (`self.TrainSpawnTransform`))
  ;[1 1 1] Set spawn position and final position on Y axis to lerp to
  (if (`|EnumEquality` ArrivalStatus "NewEnumerator2")
    ;;[1 1 1] Set Spawn Location
    (set `self.TrainSpawnTransform` (`self.NorthboundTransform`))
    ;;[1 1 1] Set Arrival Target Position
    (set `self.ArrivalTargetPos` (`self.NorthboundArrivalPos`))
    ;;[1 1 1] Set Departure Target Position
    (set `self.DepartureTargetPos` (`self.NorthboundDepPos`))
    (bind _returnvalue (`|SpawnActorFromClass` "/Game/Blueprints/Player2/BP_TrainModel.BP_TrainModel_C" _trainspawntransform "Undefined" "OverrideRootScale" null null :!label _label))
    (return _returnvalue _trainspawntransform (`self.ArrivalTargetPos`) (`self.DepartureTargetPos`))
    (elif (`|EnumEquality` ArrivalStatus "NewEnumerator3")
      (set `self.TrainSpawnTransform` (`self.SoutboundTransform`))
      (set `self.ArrivalTargetPos` (`self.SouthboundArrivalPos`))
      (set `self.DepartureTargetPos` (`self.SouthboundDepPos`))
      (goto _label)
      (elif (`|EnumEquality` ArrivalStatus "NewEnumerator0")
        (set `self.TrainSpawnTransform` (`self.NorthTermTransform`))
        (set `self.ArrivalTargetPos` (`self.NorthTermArrivalPos`))
        (set `self.DepartureTargetPos` (`self.NorthTermDepPos`))
        (goto _label)
        (elif (`|EnumEquality` ArrivalStatus "NewEnumerator1")
          (set `self.TrainSpawnTransform` (`self.SouthTermTransform`))
          (set `self.ArrivalTargetPos` (`self.SouthTermArrivalPos`))
          (set `self.DepartureTargetPos` (`self.SouthTermDepPos`))
          (goto _label))))))

(fn `TrainArrival`
  (params (TrainToArrive :type "/Game/TrainData/BP_TrainObject Object Reference") (CurrentStation :type "/Game/TrainData/E_Stations Enum" :default "NewEnumerator0"))
  (returns (ArrivalStatus :type "/Game/Blueprints/Player2/E_ArrivalStatus Enum"))
  (bind _route (`/Game/TrainData/BP_TrainObject.Route` TrainToArrive))
  (bind _returnvalue (`|EnumEquality` (`/Game/TrainData/BP_StationObject.Station` (`|GetArrayItem` _route (`KismetArrayLibrary.Array_LastIndex` _route))) CurrentStation))
  ;[1 1 1] Is TrainToArrive Westbound?
  (if (`/Game/TrainData/BP_TrainObject.Westbound` TrainToArrive)
    ;[1 1 1] Is terminating
    (if _returnvalue
      (set `self.ArrivalStatus` "NewEnumerator0")
      (else
        (set `self.ArrivalStatus` "NewEnumerator2")))
    (elif _returnvalue
      (set `self.ArrivalStatus` "NewEnumerator1")
      (else
        (set `self.ArrivalStatus` "NewEnumerator3"))))
  (return (`self.ArrivalStatus`)))

(fn `UserConstructionScript`)