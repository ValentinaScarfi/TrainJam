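; BP_TrainManager sets up the train simulation, creating randomized trains and station objects and keeping an in-game clock.
; BeginPlay fills Trains with randomized number, color, company, route and timing data, then builds one positioned station per E_Stations entry.
; The start/terminate equality check rolls separately from the returned stations, and a match leaves that train unset.
; Tick approximates whole-second pulses from real time, periodically advancing InGameTime by TimeMultiplier.
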(event `self.ReceiveBeginPlay`
  (bind _stationtoset (`self.StationToSet`))
  (for _ (range (+ (`self.NumberOfTrains`) 1))
    ;[1 1 1] Contstruct a BP_TrainObject and add it to the Trains array
    (bind _returnvalue (`|GenericCreateObject` "/Game/TrainData/BP_TrainObject.BP_TrainObject_C" self))
    ;[1 1 1] Generate a random train
    (`self.GenerateRandomTrain` _returnvalue)
    (`KismetArrayLibrary.Array_Add` (`self.Trains`) _returnvalue)
    (bind (_train_trainnumber _train_trainlength _train_traincolor _train_traincompany _train_capacity _train_startstation) (break `/Game/TrainData/Struct_Train` (`/Game/TrainData/BP_TrainObject.Train` _returnvalue)))
    ;[1 1 1] Print train number and start station
    (`KismetSystemLibrary.PrintString` (`KismetStringLibrary.Conv_IntToString` _train_trainnumber) true true (struct :`G` 0.66 :`B` 1.0 :`A` 1.0) 10.0)
    (`KismetSystemLibrary.PrintString` (`|GetEnumeratorNameAsString` _train_startstation) true true (struct :`R` 1.0 :`B` 0.115882 :`A` 1.0) 10.0))
  ;[1 1 1] Resize Stations array to length of E_Stations enum
  (`KismetArrayLibrary.Array_Resize` (`self.Stations`) (enumcount `/Game/TrainData/E_Stations`))
  ;[1 1 1] Loop through the array and construct an object for each index
  (for (_ _array_index) (`self.Stations`)
    (bind _returnvalue_2 (`|GenericCreateObject` "/Game/TrainData/BP_StationObject.BP_StationObject_C" self))
    ;[1 1 1] Set the array element to be the newly constructed object and set its Station and Position variables
    (bind _output_get (set `self.StationToSet` _returnvalue_2))
    (`KismetArrayLibrary.Array_Set` (`self.Stations`) _array_index _output_get)
    (set `/Game/TrainData/BP_StationObject.Station` (cast `/Game/TrainData/E_Stations` (`KismetMathLibrary.Conv_IntToByte` _array_index)) _stationtoset)
    (set `/Game/TrainData/BP_StationObject.Position` (`|GetArrayItem` (`self.Positions`) _array_index) _stationtoset))
  ;[1 1 1] Print to screen for debugging
  (if (`self.Debug`)
    (for _array_element (`self.Stations`)
      (bind _asbp_station_object (cast `/Game/TrainData/BP_StationObject` _array_element))
      (`KismetSystemLibrary.PrintString` (`|GetEnumeratorNameAsString` (`/Game/TrainData/BP_StationObject.Station` _asbp_station_object)) false true (struct :`G` 0.66 :`B` 1.0 :`A` 1.0) 100.0)
      (`KismetSystemLibrary.PrintString` (`KismetStringLibrary.Conv_IntToString` (`/Game/TrainData/BP_StationObject.Position` _asbp_station_object)) false true (struct :`R` 1.0 :`G` 0.061979 :`B` 0.091826 :`A` 1.0) 100.0))))

(event `self.ReceiveTick`
  (params (DeltaSeconds :type "Float (single-precision)"))
  ;[1 1 1] Timers
  (if (`KismetMathLibrary.NearlyEqual_FloatFloat` (mod (`GameplayStatics.GetRealTimeSeconds`) 1.0) 0.0 0.01)
    (set `self.TimeCounter` (+ (`self.TimeCounter`) 1))
    (if (>= (`self.TimeCounter`) 5)
      (set `self.TimeCounter` 0)
      (set `self.InGameTime` (+ (`self.InGameTime`) (`self.TimeMultiplier`))))))

(fn `GenerateRandomTrain`
  (params (TrainObject :type "/Game/TrainData/BP_TrainObject Object Reference"))
  (bind _positions (`self.Positions`))
  (bind _returnvalue (`KismetMathLibrary.RandomIntegerInRange` 0 (enumcount `/Game/TrainData/E_TrainCompanies`)))
  (bind _returnvalue_2 (`KismetMathLibrary.RandomIntegerInRange` 0 (enumcount `/Game/TrainData/E_TrainColors`)))
  (bind _returnvalue_3 (* (`KismetMathLibrary.RandomIntegerInRange` 140 340) 5))
  (bind (_isequal _startstation _terminatestation) (`self.GenerateStartAndTerminate`))
  (if _isequal
    (`KismetSystemLibrary.PrintString` "IsEqual" false true (struct :`G` 0.66 :`B` 1.0 :`A` 1.0) 10.0)
    (else
      (`KismetSystemLibrary.PrintString` "IsNotEqual" false true (struct :`G` 0.66 :`B` 1.0 :`A` 1.0) 10.0)
      (set `/Game/TrainData/BP_TrainObject.Train` (make `/Game/TrainData/Struct_Train` (`KismetMathLibrary.RandomIntegerInRange` 1000 9999) (`KismetMathLibrary.RandomIntegerInRange` 1 5) (cast `/Game/TrainData/E_TrainColors` (`KismetMathLibrary.Conv_IntToByte` _returnvalue_2)) (cast `/Game/TrainData/E_TrainCompanies` (`KismetMathLibrary.Conv_IntToByte` _returnvalue)) (`KismetMathLibrary.RandomIntegerInRange` 50 400) _startstation _terminatestation _returnvalue_3 (+ (`KismetMathLibrary.Abs_Int` (- (`|GetArrayItem` _positions _returnvalue_2) (`|GetArrayItem` _positions _returnvalue))) _returnvalue_3)) TrainObject))))

(fn `GenerateStartAndTerminate`
  (returns (IsEqual :type Boolean) (StartStation :type "/Game/TrainData/E_Stations Enum") (TerminateStation :type "/Game/TrainData/E_Stations Enum"))
  (bind _returnvalue (cast `/Game/TrainData/E_Stations` (`KismetMathLibrary.Conv_IntToByte` (`KismetMathLibrary.RandomIntegerInRange` 0 (enumcount `/Game/TrainData/E_Stations`)))))
  (bind _returnvalue_2 (cast `/Game/TrainData/E_Stations` (`KismetMathLibrary.Conv_IntToByte` (`KismetMathLibrary.RandomIntegerInRange` 0 (enumcount `/Game/TrainData/E_Stations`)))))
  (return (`|EnumEquality` _returnvalue_2 _returnvalue) _returnvalue_2 _returnvalue))

(fn `GetDistance`
  (params (StartStation :type "/Game/TrainData/BP_StationObject Object Reference") (EndStation :type "/Game/TrainData/BP_StationObject Object Reference"))
  (returns (JourneyTime :type Integer))
  (return (`KismetMathLibrary.Abs_Int` (- (`/Game/TrainData/BP_StationObject.Position` StartStation) (`/Game/TrainData/BP_StationObject.Position` EndStation)))))

(fn `UserConstructionScript`)